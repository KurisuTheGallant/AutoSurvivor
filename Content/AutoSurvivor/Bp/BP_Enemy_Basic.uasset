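; BP_Enemy_Basic is the basic enemy Blueprint for AutoSurvivor, and its graph handles visual feedback when it takes damage.
; OnDamageReceived creates a WBP_DamageText widget with the amount, placed at the enemy's location projected to screen space.
; After a tiny delay it spawns a half-scale spark emitter at the hit location.
; A DoOnce that resets after a short delay throttles the feedback, so rapid hits in that window show nothing.
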(event EventOnDamageReceived
  (params (Amount :type Float%20%28single-precision%29) (HitLocation :type Vector :default "0, 0, 0"))
  (bind _returnvalue (Game|GetPlayerController 0))
  (Utilities|FlowControl|DoOnce false :!label _label
    (:Completed
      (bind _returnvalue_2 (UserInterface|CreateWidget "/Game/AutoSurvivor/widget/WBP_DamageText.WBP_DamageText_C" _returnvalue))
      (Default|InitDamageText _returnvalue_2 Amount)
      (UserInterface|Viewport|AddtoViewport _returnvalue_2 0)
      (Class|UserWidget|SetPositioninViewport _returnvalue_2 (.ScreenPosition (Class|GameplayStatics|ProjectWorldtoScreen _returnvalue (Transformation|GetActorLocation) false)) false)
      (Utilities|FlowControl|Delay 0.01)
      (Effects|SpawnEmitteratLocation "/Game/Realistic_Starter_VFX_Pack_Vol2/Particles/Sparks/P_Sparks_C.P_Sparks_C" HitLocation "0, 0, 0" "0.500000,0.500000,0.500000")
      (Utilities|FlowControl|Delay 0.2)
      (goto _label Reset))))

(fn ConstructionScript)